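; Squad controller for Human1 soldiers in an RTS that spawns the units and commands them as one group.
; BeginPlay spawns an initial squad, and SpawnUnit adds soldiers until a reinforcement counter runs out.
; Each new soldier appears randomly inside the last unit's SpawnerCheck bounds and gets a reference to this controller.
; SetWidget binds the controller to the player's unit UI, while SetPosition relays move orders to every soldier.
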(event Custom|SetWidget
  (bind _asbp_rtstest (Utilities|Casting|CastToBP_RTSTest (Game|Player|GetPlayerPawn 0)))
  (Class|WidgetSwitcher|SetActiveWidgetIndex (Variables|/Game/Blueprint/UI/UI_General.UI_General_C|GetWidgetSwitcher_General (Variables|/Game/Blueprint/PlayerTest/BP_RTSTest.BP_RTSTest_C|GetUI_General _asbp_rtstest)) 2)
  (Variables|/Game/Blueprint/UI/UI_Unit.UI_Unit_C|SetMasterControler (Variables|/Game/Blueprint/UI/UI_General.UI_General_C|GetUI_Unit (Variables|/Game/Blueprint/PlayerTest/BP_RTSTest.BP_RTSTest_C|GetUI_General _asbp_rtstest)) self))

(event Custom|SetPosition
  (params (PositionSelect :type Vector))
  (for _array_element (Variables|Default|GetUnitSpawn)
    (Default|GotoPosition (Variables|/Game/Blueprint/Human1/Soldier/BP_Humain1_Soldier.BP_Humain1_Soldier_C|GetControlerUnitRef _array_element) PositionSelect)))

(event Custom|SpawnUnit
  (if (!= (Variables|Default|GetLeftUnitToSpawn) 0)
    (Variables|Default|SetLeftUnitToSpawn (Math|Integer|Clamp(Integer) (- (Variables|Default|GetLeftUnitToSpawn) 1) 0 4))
    (for _array_element (Variables|Default|GetUnitSpawn)
      _)
    (bind _returnvalue (Game|SpawnActorfromClass "/Game/Blueprint/Human1/Soldier/BP_Humain1_Soldier.BP_Humain1_Soldier_C" (Math|Transform|MakeTransform (Math|Random|RandomPointinBoundingBox (.Origin (Collision|GetComponentBounds (Variables|/Game/Blueprint/Human1/Soldier/BP_Humain1_Soldier.BP_Humain1_Soldier_C|GetSpawnerCheck _array_element))) (.BoxExtent (Collision|GetComponentBounds (Variables|/Game/Blueprint/Human1/Soldier/BP_Humain1_Soldier.BP_Humain1_Soldier_C|GetSpawnerCheck _array_element)))) "0, 0, 0" "1.000000,1.000000,1.000000") "AdjustIfPossibleButAlwaysSpawn" "MultiplyWithRoot" 0 0))
    (Variables|/Game/Blueprint/Human1/Soldier/BP_Humain1_Soldier.BP_Humain1_Soldier_C|SetControlerRef _returnvalue self)
    (Utilities|Array|Add (Variables|Default|GetUnitSpawn) _returnvalue)))

(event EventBeginPlay
  (Utilities|FlowControl|Sequence
    (:then_0
      (bind _returnvalue (Game|SpawnActorfromClass "/Game/Blueprint/Human1/Soldier/BP_Humain1_Soldier.BP_Humain1_Soldier_C" (Math|Transform|MakeTransform (Transformation|GetActorLocation) (Transformation|GetActorRotation) "1.000000,1.000000,1.000000") "Undefined" "MultiplyWithRoot" 0 0))
      (Variables|/Game/Blueprint/Human1/Soldier/BP_Humain1_Soldier.BP_Humain1_Soldier_C|SetControlerRef _returnvalue self)
      (Utilities|Array|Add (Variables|Default|GetUnitSpawn) _returnvalue)
      (Variables|Default|SetLeftUnitToSpawn 4))
    (:then_1
      (for _index (range 0 2)
        (for _array_element (Variables|Default|GetUnitSpawn)
          _)
        (bind _returnvalue_2 (Game|SpawnActorfromClass "/Game/Blueprint/Human1/Soldier/BP_Humain1_Soldier.BP_Humain1_Soldier_C" (Math|Transform|MakeTransform (Math|Random|RandomPointinBoundingBox (.Origin (Collision|GetComponentBounds (Variables|/Game/Blueprint/Human1/Soldier/BP_Humain1_Soldier.BP_Humain1_Soldier_C|GetSpawnerCheck _array_element))) (.BoxExtent (Collision|GetComponentBounds (Variables|/Game/Blueprint/Human1/Soldier/BP_Humain1_Soldier.BP_Humain1_Soldier_C|GetSpawnerCheck _array_element)))) "0, 0, 0" "1.000000,1.000000,1.000000") "AdjustIfPossibleButAlwaysSpawn" "MultiplyWithRoot" 0 0))
        (Variables|/Game/Blueprint/Human1/Soldier/BP_Humain1_Soldier.BP_Humain1_Soldier_C|SetControlerRef _returnvalue_2 self)
        (Utilities|Array|Add (Variables|Default|GetUnitSpawn) _returnvalue_2)))))

(fn ConstructionScript)