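; BP_RTSTest is a test RTS-style camera pawn driven by Enhanced Input through IMC_Camera.
; Input actions move it along the root's forward and right axes, yaw the root, and tilt the SpringArm within a clamped pitch.
; Each tick, a debug-drawn forward trace from the camera sets arm length to a base plus the hit normal's Z, printing location and length, or resets it on a miss.
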(event Input|EnhancedActionEvents|EnhancedInputActionIA_CamUpAndDown
  (params (ActionValue :type Float%20%28double-precision%29) (ElapsedSeconds :type Float%20%28double-precision%29) (TriggeredSeconds :type Float%20%28double-precision%29) (InputAction :type Input%20Action%20Object%20Reference :default "/Game/Blueprint/Input/InputAction/CamInput/IA_CamUpAndDown.IA_CamUpAndDown"))
  (Pawn|Input|AddMovementInput (Math|Vector|GetForwardVector (Variables|Default|GetDefaultSceneRoot)) ActionValue false))

(event Input|EnhancedActionEvents|EnhancedInputActionIA_CamLeftAndRight
  (params (ActionValue :type Float%20%28double-precision%29) (ElapsedSeconds :type Float%20%28double-precision%29) (TriggeredSeconds :type Float%20%28double-precision%29) (InputAction :type Input%20Action%20Object%20Reference :default "/Game/Blueprint/Input/InputAction/CamInput/IA_CamLeftAndRight.IA_CamLeftAndRight"))
  (Pawn|Input|AddMovementInput (Math|Vector|GetRightVector (Variables|Default|GetDefaultSceneRoot)) ActionValue false))

(event Input|EnhancedActionEvents|EnhancedInputActionIA_CamRotationLeftAndRight
  (params (ActionValue :type Float%20%28double-precision%29) (ElapsedSeconds :type Float%20%28double-precision%29) (TriggeredSeconds :type Float%20%28double-precision%29) (InputAction :type Input%20Action%20Object%20Reference :default "/Game/Blueprint/Input/InputAction/CamInput/IA_CamRotationLeftAndRight.IA_CamRotationLeftAndRight"))
  (bind _defaultsceneroot (Variables|Default|GetDefaultSceneRoot))
  (bind _returnvalue (Transformation|GetWorldRotation _defaultsceneroot))
  (bind (_roll _pitch _yaw) (Math|Rotator|BreakRotator _returnvalue))
  (Transformation|SetWorldRotation _defaultsceneroot (Math|Rotator|MakeRotator _roll _pitch (+ _yaw ActionValue)) false false))

(event Input|EnhancedActionEvents|EnhancedInputActionIA_CamInclinaisonUpAndDown
  (params (ActionValue :type Float%20%28double-precision%29) (ElapsedSeconds :type Float%20%28double-precision%29) (TriggeredSeconds :type Float%20%28double-precision%29) (InputAction :type Input%20Action%20Object%20Reference :default "/Game/Blueprint/Input/InputAction/CamInput/IA_CamInclinaisonUpAndDown.IA_CamInclinaisonUpAndDown"))
  (bind _springarm (Variables|Default|GetSpringArm))
  (bind _returnvalue (Transformation|GetWorldRotation _springarm))
  (bind (_roll _pitch _yaw) (Math|Rotator|BreakRotator _returnvalue))
  (Transformation|SetWorldRotation _springarm (Math|Rotator|MakeRotator _roll (Math|Float|Clamp(Float) (+ _pitch ActionValue) -75.0 -25.0) _yaw) false false))

(event EventBeginPlay
  (Input|AddMappingContext (PlayerController|LocalPlayerSubsystems|GetEnhancedInputLocalPlayerSubsystem (Game|GetPlayerController 0)) "/Game/Blueprint/Input/IMC_Camera.IMC_Camera" 0 "(bIgnoreAllPressedKeysUntilRelease=True,bForceImmediately=False,bNotifyUserSettings=False)"))

(event EventTick
  (params (DeltaSeconds :type Float%20%28single-precision%29))
  (bind _camera (Variables|Default|GetCamera))
  (bind _springarm (Variables|Default|GetSpringArm))
  (bind _returnvalue (Transformation|GetWorldLocation _camera))
  (bind (_outhit _returnvalue_2) (Collision|LineTraceByChannel _returnvalue (+ _returnvalue (* (Math|Vector|GetForwardVector (Transformation|GetWorldRotation _camera)) 6.5e+02)) "TraceTypeQuery1" false 0 "ForOneFrame"))
  (if _returnvalue_2
    (Variables|/Script/Engine.SpringArmComponent|SetTargetArmLength _springarm (+ (.Z (Math|Vector|BreakVector (.Normal (Collision|BreakHitResult _outhit)))) 6e+02))
    (Development|PrintString (Utilities|String|ToString(Vector) (Transformation|GetActorLocation)) true true "(R=0.000000,G=0.660000,B=1.000000,A=1.000000)" 0.0)
    (Development|PrintString (Utilities|String|ToString(Float) (Variables|/Script/Engine.SpringArmComponent|GetTargetArmLength (Variables|Default|GetSpringArm))) true true "(R=0.057249,G=1.000000,B=0.000000,A=1.000000)" 0.0)
    (else
      (Variables|/Script/Engine.SpringArmComponent|SetTargetArmLength _springarm 6e+02))))

(fn ConstructionScript)